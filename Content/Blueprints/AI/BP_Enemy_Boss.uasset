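; Boss enemy Blueprint that handles the telegraph and aiming of a charge attack.
; Charge sets state flags, plays a scream montage and opens a Tick gate until the montage completes.
; While gated, a debug-drawn, capsule-radius sphere trace runs level toward the player, storing its hit location as EndCharge.
; The montage notify plays a howl and switches aim from the player to the stored EndCharge.
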(event `self.GetHitAnim`
  (params (MontageToPlay :type "AnimMontage Object Reference") (AkEvent :type "AkAudioEvent Object Reference")))

(event `self.ReceiveTick`
  (params (DeltaSeconds :type "Float (single-precision)"))
  (bind (_returnvalue_x _returnvalue_y) (`KismetMathLibrary.BreakVector` (`self.K2_GetActorLocation`)))
  (bind _returnvalue (`KismetMathLibrary.SelectVector` (`self.EndCharge`) (`self.K2_GetActorLocation` (`GameplayStatics.GetPlayerCharacter` 0)) (not (`self.Screaming?`))))
  (bind _returnvalue_2 (`KismetMathLibrary.MakeVector` _returnvalue_x _returnvalue_y (.z _returnvalue)))
  (`parent.ReceiveTick` DeltaSeconds)
  (`/Engine/EditorBlueprintResources/StandardMacros.Gate` true :!label _label
    (:`Exit`
      (bind _outhit (`KismetSystemLibrary.SphereTraceSingleForObjects` :`Start` _returnvalue_2 :`End` (+ _returnvalue_2 (* (`KismetMathLibrary.GetDirectionUnitVector` _returnvalue_2 _returnvalue) 20000.0)) :`Radius` (`CapsuleComponent.GetScaledCapsuleRadius` (`self.CapsuleComponent`)) :`ObjectTypes` (`|MakeArray` "ObjectTypeQuery3" "ObjectTypeQuery1" :!type "EObjectTypeQuery Enum") :`DrawDebugType` "ForOneFrame"))
      (set `self.EndCharge` (`.Location` (`GameplayStatics.BreakHitResult` _outhit))))))

(event `Charge`
  (set `self.Charge?` true)
  (set `self.Screaming?` true)
  (`|PlayMontage` (`self.Mesh`) "/Game/Enemy/Boss/Animations/Zombie_Scream_Montage.Zombie_Scream_Montage"
    (:`then`
      (goto _label :!via `Open`))
    (:`OnCompleted`
      (goto _label :!via `Close`))
    (:`OnNotifyBegin`
      (set `self.Screaming?` false)
      (`AkGameplayStatics.PostEvent` "/Game/WwiseAudio/Events/Raphael_Work_Unit/Play_howl.Play_howl" self))))

(fn `UserConstructionScript`
  (`parent.UserConstructionScript`))