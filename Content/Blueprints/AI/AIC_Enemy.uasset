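; AIC_Enemy is an enemy AI controller that starts a behavior tree and supplies its blackboard targets.
; LaunchIA runs the behavior tree passed to it, then stores the first player's character as PlayerRef.
; NextResource removes the given entry from the TabResources array, then sets ResourceRef to the first remaining one or clears it when none are left.
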(event `LaunchIA`
  (params (BTAsset :type "BehaviorTree Object Reference"))
  (`self.RunBehaviorTree` BTAsset)
  (`BlackboardComponent.SetValueAsObject` (`self.Blackboard`) (`KismetStringLibrary.Conv_StringToName` "PlayerRef") (`GameplayStatics.GetPlayerCharacter` 0)))

(event `NextResource`
  (params (Key :type "/Game/Blueprints/BP_Resource Object Reference (by ref)"))
  (bind _tabresources (`self.TabResources`))
  (`KismetArrayLibrary.Array_RemoveItem` _tabresources Key)
  (if (> (`KismetArrayLibrary.Array_Length` _tabresources) 0)
    (`BlackboardComponent.SetValueAsObject` (`self.Blackboard`) (`KismetStringLibrary.Conv_StringToName` "ResourceRef") (`|GetArrayItem` (`self.TabResources`)))
    (else
      (`BlackboardComponent.ClearValue` (`self.Blackboard`) (`KismetStringLibrary.Conv_StringToName` "ResourceRef")))))

(fn `UserConstructionScript`)