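; AnimNotifyState_Attack is a melee hit-detection notify state for the attack animations of BP_EnemyCaC.
; Each tick, while the enemy's PlayerHit flag is false, it sphere-traces pawns between the LeftArm and LeftHandMiddle4 sockets, with debug drawing on.
; If the trace hits BP_Player, it applies fixed damage and sets PlayerHit, which blocks further hits; this notify never resets the flag.
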(fn `Received_NotifyTick`
  (params (MeshComp :type "SkeletalMeshComponent Object Reference") (Animation :type "AnimSequenceBase Object Reference") (FrameDeltaTime :type "Float (double-precision)"))
  (returns (ReturnValue :type Boolean))
  (locals (EnemyRef :type "/Game/Blueprints/AI/BP_EnemyCaC Object Reference"))
  (bind _asbp_enemy_ca_c (cast `/Game/Blueprints/AI/BP_EnemyCaC` (`ActorComponent.GetOwner` MeshComp)))
  (bind _output_get (set `local.EnemyRef` _asbp_enemy_ca_c))
  (if (not (`/Game/Blueprints/AI/BP_EnemyCaC.PlayerHit?` _output_get))
    (bind _outhit (`KismetSystemLibrary.SphereTraceSingleForObjects` :`WorldContextObject` MeshComp :`Start` (`SceneComponent.GetSocketLocation` MeshComp "LeftArm") :`End` (`SceneComponent.GetSocketLocation` MeshComp "LeftHandMiddle4") :`Radius` 10.0 :`ObjectTypes` (`|MakeArray` "ObjectTypeQuery3" :!type "EObjectTypeQuery Enum") :`DrawDebugType` "ForDuration"))
    (bind _asbp_player (cast `/Game/Blueprints/BP_Player` (`.HitActor` (`GameplayStatics.BreakHitResult` _outhit))))
    (`GameplayStatics.ApplyDamage` _asbp_player 10.0)
    (set `/Game/Blueprints/AI/BP_EnemyCaC.PlayerHit?` true (`local.EnemyRef`))
    (return true)))