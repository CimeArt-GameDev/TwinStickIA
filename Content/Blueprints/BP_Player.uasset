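; Twin-stick shooter player character with camera-relative movement, health and wave kill tracking that relaunches the spawner.
; Tick slowly rotates the spring arm, turns the player toward fire-axis input, auto-fires and prints debug stats.
; Firing line-traces from the pistol muzzle with a Niagara beam and delay-gated cooldown, damaging enemies by weapon flag.
; A timed, retriggerable OS mode swaps the beam effect and massively boosts damage.
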(event `InputAxis|MoveForward`
  (params (AxisValue :type "Float (single-precision)"))
  (bind (_returnvalue_x _returnvalue_y) (`KismetMathLibrary.BreakVector` (`SceneComponent.GetForwardVector` (`self.Camera1`))))
  (`self.AddMovementInput` (`KismetMathLibrary.Normal` (`KismetMathLibrary.MakeVector` _returnvalue_x _returnvalue_y)) AxisValue))

(event `InputAxis|MoveRight`
  (params (AxisValue :type "Float (single-precision)"))
  (bind (_returnvalue_x _returnvalue_y) (`KismetMathLibrary.BreakVector` (`SceneComponent.GetRightVector` (`self.Camera1`))))
  (`self.AddMovementInput` (`KismetMathLibrary.Normal` (`KismetMathLibrary.MakeVector` _returnvalue_x _returnvalue_y)) AxisValue))

(event `self.ReceiveTick`
  (params (DeltaSeconds :type "Float (single-precision)"))
  (bind (_returnvalue_roll _returnvalue_pitch _returnvalue_yaw) (`KismetMathLibrary.BreakRotator` (`KismetMathLibrary.FindLookAtRotation` (0.0 0.0 0.0) (`KismetMathLibrary.GreaterGreater_VectorRotator` (`KismetMathLibrary.MakeVector` (`self.GetInputAxisValue`) (`self.GetInputAxisValue`)) (`KismetMathLibrary.MakeRotFromX` (`SceneComponent.GetForwardVector` (`self.Camera1`)))))))
  (`|ExecutionSequence`
    (:`then_0`
      (`SceneComponent.K2_AddRelativeRotation` (`self.SpringArm1`) (struct :`Yaw` 0.05) false false))
    (:`then_1`
      (bind _output_get (set `CharacterMovementComponent.bOrientRotationToMovement` (and (`KismetMathLibrary.NearlyEqual_FloatFloat` (`self.GetInputAxisValue`)) (`KismetMathLibrary.NearlyEqual_FloatFloat` (`self.GetInputAxisValue`))) (`self.CharacterMovement`)))
      (if (not _output_get)
        (`Controller.SetControlRotation` (`GameplayStatics.GetPlayerController` 0) (`KismetMathLibrary.MakeRotator` 0.0 0.0 _returnvalue_yaw))))
    (:`then_2`
      (`self.Fire`))
    (:`then_3`
      (`KismetSystemLibrary.PrintString` (`KismetStringLibrary.Concat_StrStr` "Health : " (`KismetStringLibrary.Conv_DoubleToString` (`self.Health`)) "    TotalKills : " (`KismetStringLibrary.Conv_IntToString` (`self.TotalKills`)) "     WaveKills : " (`KismetStringLibrary.Conv_IntToString` (`self.NbKillsWave`))) true true (struct :`G` 0.66 :`B` 1.0 :`A` 1.0) 0.001))))

(event `Fire`
  (bind _darkness_pistol (`self.Darkness_Pistol`))
  (bind _returnvalue (`SceneComponent.GetSocketLocation` (`self.Darkness_Pistol`) "Muzzle"))
  (if (and (not (`CharacterMovementComponent.bOrientRotationToMovement` (`self.CharacterMovement`))) (`self.CanFire?`))
    (bind _outhit (`KismetSystemLibrary.LineTraceSingleForObjects` _returnvalue (+ _returnvalue (* (`self.GetActorForwardVector`) 200000.0)) (`|MakeArray` "ObjectTypeQuery3" "ObjectTypeQuery1" :!type "EObjectTypeQuery Enum")))
    (`|ExecutionSequence`
      (:`then_0`
        (bind _returnvalue_2 (`NiagaraFunctionLibrary.SpawnSystemAtLocation` (select `bool` (`self.OSMode?`) :`false` "/Game/FX/NiagaraSystems/NS_PistolFire.NS_PistolFire" :`true` "/Game/FX/NiagaraSystems/NS_PistolOS.NS_PistolOS" :!type "NiagaraSystem Object Reference") (`SceneComponent.GetSocketLocation` _darkness_pistol "Muzzle") (`SceneComponent.GetSocketRotation` _darkness_pistol "Muzzle")))
        (`FXSystemComponent.SetVectorParameter` _returnvalue_2 "BeamStart" (`SceneComponent.GetSocketLocation` (`self.Darkness_Pistol`) "Muzzle"))
        (`FXSystemComponent.SetVectorParameter` _returnvalue_2 "BeamEnd" (`.ImpactPoint` (`GameplayStatics.BreakHitResult` _outhit)))
        (`SkeletalMeshComponent.PlayAnimation` (`self.Darkness_Pistol`) "/Game/Weapons/Meshes/Anims/Fire_Pistol_W.Fire_Pistol_W" false)
        (set `self.CanFire?` false)
        (`KismetSystemLibrary.Delay` 0.5)
        (set `self.CanFire?` true))
      (:`then_1`
        (bind _asbp_enemy (cast `/Game/Blueprints/AI/BP_Enemy` (`.HitActor` (`GameplayStatics.BreakHitResult` _outhit))))
        (`GameplayStatics.ApplyDamage` _asbp_enemy (`KismetMathLibrary.SelectFloat` 5000.0 (`KismetMathLibrary.SelectFloat` 50.0 20.0 (`self.Shotgun?`)) (`self.OSMode?`)))))))

(event `self.ReceiveAnyDamage`
  (params (Damage :type "Float (single-precision)") (DamageType :type "DamageType Object Reference") (InstigatedBy :type "Controller Object Reference") (DamageCauser :type "Actor Object Reference"))
  (set `self.Health` (- (`self.Health`) Damage))
  (`/Game/Player/Animations/AnimBP_Player.GetHitAnim` (cast `/Game/Player/Animations/AnimBP_Player` (`SkeletalMeshComponent.GetAnimInstance` (`self.Mesh`)) :!pure true)))

(event `ActivateOSMode`
  (set `self.OSMode?` true)
  (`KismetSystemLibrary.RetriggerableDelay` 15.0)
  (set `self.OSMode?` false))

(event `self.ReceiveBeginPlay`
  (bind _returnvalue (`GameplayStatics.GetActorOfClass` "/Game/Blueprints/BP_Spawner.BP_Spawner_C"))
  (set `self.SpawnerRef` _returnvalue))

(event `IncrementKills`
  (bind _result (`/Engine/EditorBlueprintResources/StandardMacros.IncrementInt` (`self.NbKillsWave`))
    (:`  `
      (`/Engine/EditorBlueprintResources/StandardMacros.IncrementInt` (`self.TotalKills`)
        (:`  `
          (if (>= _result (`/Game/Blueprints/BP_Spawner.EnemiesPerWaves` (`self.SpawnerRef`)))
            (set `self.NbKillsWave` 0)
            (`/Game/Blueprints/BP_Spawner.RelaunchSpawn` (`self.SpawnerRef`))))))))

(fn `UserConstructionScript`)