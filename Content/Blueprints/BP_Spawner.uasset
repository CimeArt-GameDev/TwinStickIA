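; Enemy wave spawner actor that fills a box area with random enemy classes until the wave count is reached.
; A looping timer traces down from random box points and spawns at the hit point, adjusting for collisions.
; Only enemies with a successful navigation path query to the player count; others are destroyed.
; RelaunchSpawn resets the count, scales up the wave size and resumes the timer, which pauses when full.
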(event `self.ReceiveBeginPlay`
  (bind _returnvalue (`KismetSystemLibrary.K2_SetTimerDelegate` (delegate `SpawnMobs`) 0.1 true))
  (set `self.SpawnHandler` _returnvalue))

(event `SpawnMobs`
  (bind _box (`self.Box`))
  (bind _enemyclasses (`self.EnemyClasses`))
  (bind _returnvalue (`SceneComponent.K2_GetComponentLocation` _box))
  (bind (_returnvalue_x _returnvalue_y _returnvalue_z) (`KismetMathLibrary.BreakVector` (`KismetMathLibrary.RandomPointInBoundingBox` _returnvalue (`BoxComponent.BoxExtent` _box))))
  (bind _returnvalue_2 (+ (.z _returnvalue) (/ _returnvalue_z 2.0)))
  (if (< (`self.NbMobs`) (`self.EnemiesPerWaves`))
    (bind _outhit (`KismetSystemLibrary.LineTraceSingle` :`Start` (`KismetMathLibrary.MakeVector` _returnvalue_x _returnvalue_y _returnvalue_2) :`End` (`KismetMathLibrary.MakeVector` _returnvalue_x _returnvalue_y (- _returnvalue_2 1000.0)) :`TraceChannel` "TraceTypeQuery1" :`DrawDebugType` "Persistent"))
    (bind _returnvalue_3 (`|SpawnActorFromClass` (`|GetArrayItem` _enemyclasses (`KismetMathLibrary.RandomIntegerInRange` 0 (`KismetArrayLibrary.Array_LastIndex` _enemyclasses))) (`KismetMathLibrary.MakeTransform` (`.ImpactPoint` (`GameplayStatics.BreakHitResult` _outhit))) "AdjustIfPossibleButDontSpawnIfColliding" "OverrideRootScale" null null))
    (`/Engine/EditorBlueprintResources/StandardMacros.IsValid` _returnvalue_3
      (:`Is Valid`
        (if (`|EnumEquality` (`.ReturnValue` (`NavigationSystemV1.GetPathLength` (`.ImpactPoint` (`GameplayStatics.BreakHitResult` _outhit)) (`self.K2_GetActorLocation` (`GameplayStatics.GetPlayerCharacter` 0)) null null)) "Success")
          (`/Engine/EditorBlueprintResources/StandardMacros.IncrementInt` (`self.NbMobs`))
          (else
            (`self.K2_DestroyActor` _returnvalue_3)))))
    (else
      (`KismetSystemLibrary.K2_PauseTimerHandle` (`self.SpawnHandler`)))))

(event `RelaunchSpawn`
  (set `self.NbMobs` 0)
  (set `self.EnemiesPerWaves` (`KismetMathLibrary.FTrunc` (* (`self.EnemiesPerWaves`) 1.2)))
  (`KismetSystemLibrary.K2_UnPauseTimerHandle` (`self.SpawnHandler`)))

(fn `UserConstructionScript`)